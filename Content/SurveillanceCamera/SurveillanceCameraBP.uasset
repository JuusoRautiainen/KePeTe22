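; Surveillance camera that detects tagged players, shows its state with a colored decal and shocks the player on alarm.
; Cone overlaps track the detected player and toggle the NewUI HUD, fetched through player controller index 5.
; State changes recolor the dynamic decal material; Alarm aims a shock effect and spawns a burst at the player, Seeking hides it, Analyzing calls an empty ShokkiOff.
; Raising the alarm notifies the HUD and calls alarm dispatch.
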(event `self.ReceiveBeginPlay`
  (bind _returnvalue (`KismetMaterialLibrary.CreateDynamicMaterialInstance` "/Game/SurveillanceCamera/AreaMaterial.AreaMaterial"))
  (bind _output_get (set `self.DecalMatsku` _returnvalue))
  (`DecalComponent.SetDecalMaterial` (`self.Decal`) _output_get))

(event `self.OnStateChange`
  (params (newState :type "CameraState Enum" :default "kSeeking"))
  (switch `CameraState` newState
    (:`kSeeking`
      (`MaterialInstanceDynamic.SetVectorParameterValue` (`self.DecalMatsku`) "Vari" (struct :`R` 0.03566 :`G` 0.113507 :`B` 0.658333 :`A` 1.0))
      (`SceneComponent.SetVisibility` (`self.Shokki`) false false))
    (:`kAnalyzing`
      (`MaterialInstanceDynamic.SetVectorParameterValue` (`self.DecalMatsku`) "Vari" (struct :`R` 0.067995 :`G` 0.807544 :`B` 0.8625 :`A` 1.0))
      (`self.ShokkiOff`))
    (:`kAlarm`
      (`MaterialInstanceDynamic.SetVectorParameterValue` (`self.DecalMatsku`) "Vari" (struct :`R` 0.970833 :`G` 0.03392 :`B` 0.00809 :`A` 1.0))
      (`self.ShokkiPelaaja`))))

(event `self.SurveillanceCone.OnComponentBeginOverlap`
  (params (OverlappedComponent :type "PrimitiveComponent Object Reference") (OtherActor :type "Actor Object Reference") (OtherComp :type "PrimitiveComponent Object Reference") (OtherBodyIndex :type Integer) (bFromSweep :type Boolean) (SweepResult :type "HitResult Structure (by ref)"))
  (if (`self.ActorHasTag` OtherActor "Player")
    (set `self.detectedPlayer` OtherActor)
    (bind _asnew_ui (cast `/Game/HUD/NewUI` (`PlayerController.GetHUD` (`GameplayStatics.GetPlayerController` 5))))
    (`/Game/HUD/NewUI.KameranKantamanSisällä` _asnew_ui)))

(event `self.SurveillanceCone.OnComponentEndOverlap`
  (params (OverlappedComponent :type "PrimitiveComponent Object Reference") (OtherActor :type "Actor Object Reference") (OtherComp :type "PrimitiveComponent Object Reference") (OtherBodyIndex :type Integer))
  (if (`self.ActorHasTag` OtherActor "Player")
    (set `self.detectedPlayer` null)
    (bind _asnew_ui (cast `/Game/HUD/NewUI` (`PlayerController.GetHUD` (`GameplayStatics.GetPlayerController` 5))))
    (`/Game/HUD/NewUI.PiilotaNewUI` _asnew_ui)))

(event `self.OnRaiseAlarm`
  (`KismetSystemLibrary.PrintString` "Alarm")
  (bind _asnew_ui (cast `/Game/HUD/NewUI` (`PlayerController.GetHUD` (`GameplayStatics.GetPlayerController` 5))))
  (`/Game/HUD/NewUI.LaukaiseHalytys` _asnew_ui)
  (`self.AlarmDispatch`))

(fn `ShokkiOff`)

(fn `ShokkiPelaaja`
  ;[1 1 1] Shokki kamerasta pelaajaan
  (`|ExecutionSequence`
    (:`then_0`
      (`FXSystemComponent.SetActorParameter` (`self.Shokki`) "Loppu" (`self.detectedPlayer`))
      (`SceneComponent.SetVisibility` (`self.Shokki`) true false))
    (:`then_1`
      ;[1 1 1] Pelaajan shokkiryöppy
      (bind _returnvalue (`|SpawnActorFromClass` "/Game/SahkoShokki/ShokkiRyoppyActor.ShokkiRyoppyActor_C" (`self.GetTransform` (`self.detectedPlayer`)) "Undefined" "OverrideRootScale" null null))
      (`FXSystemComponent.SetActorParameter` (`/Game/SahkoShokki/ShokkiRyoppyActor.ShokkiRyoppy` _returnvalue) "Keskus" (`self.detectedPlayer`)))))

(fn `UserConstructionScript`)